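; BP_Healer is an enemy that heals nearby BP_Melee and BP_Ranged actors.
; Tick refreshes its health widget, then a one-second Delay paces healing of actors overlapping SphereHealingCollider, capped at their MaxHP.
; BeginPlay sets starting health and the widget maximum.
; PlayerProjectile hits deduct fixed damage and destroy the healer when health runs out.
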(event `self.ReceiveBeginPlay`
  (bind _returnvalue (`EnemyHealth.SetHealth` "EType_Healer"))
  (set `self.health` _returnvalue)
  (bind _asuienemy_health (cast `/Game/BluePrints/UIEnemyHealth` (`WidgetComponent.GetUserWidgetObject` (`self.UIWidget`))))
  (bind _output_get (set `self.BP HealthWidget` _asuienemy_health))
  (set `/Game/BluePrints/UIEnemyHealth.maxHealth` (`self.health`) _output_get))

(event `self.ReceiveTick`
  (params (DeltaSeconds :type "Float (single-precision)"))
  (bind _spherehealingcollider (`self.SphereHealingCollider`))
  (set `/Game/BluePrints/UIEnemyHealth.currentHealth` (`self.health`) (`self.BP HealthWidget`))
  (`KismetSystemLibrary.Delay` 1.0)
  (for _array_element (`PrimitiveComponent.GetOverlappingActors` _spherehealingcollider "/Game/BluePrints/BP_Melee.BP_Melee_C")
    (bind _asbp_melee (cast `/Game/BluePrints/BP_Melee` _array_element))
    (bind _health (`/Game/BluePrints/BP_Melee.Health` _asbp_melee))
    (bind _maxhp (`/Game/BluePrints/BP_Melee.MaxHP` _asbp_melee))
    (if (<= _health _maxhp)
      (bind _returnvalue (+ _health (`self.healingAmount`)))
      (if (> _returnvalue _maxhp)
        (set `/Game/BluePrints/BP_Melee.Health` _maxhp _asbp_melee)
        (else
          (set `/Game/BluePrints/BP_Melee.Health` _returnvalue _asbp_melee)))))
  (for _array_element_2 (`PrimitiveComponent.GetOverlappingActors` _spherehealingcollider "/Game/BluePrints/BP_Ranged.BP_Ranged_C")
    (bind _asbp_ranged (cast `/Game/BluePrints/BP_Ranged` _array_element_2))
    (bind _health_2 (`/Game/BluePrints/BP_Ranged.Health` _asbp_ranged))
    (bind _maxhp_2 (`/Game/BluePrints/BP_Ranged.MaxHP` _asbp_ranged))
    (if (<= _health_2 _maxhp_2)
      (bind _returnvalue_2 (+ _health_2 (`self.healingAmount`)))
      (if (> _returnvalue_2 _maxhp_2)
        (set `/Game/BluePrints/BP_Ranged.Health` _maxhp_2 _asbp_ranged)
        (else
          (set `/Game/BluePrints/BP_Ranged.Health` _returnvalue_2 _asbp_ranged))))))

(event `self.ReceiveHit`
  (params (MyComp :type "PrimitiveComponent Object Reference") (Other :type "Actor Object Reference") (OtherComp :type "PrimitiveComponent Object Reference") (bSelfMoved :type Boolean) (HitLocation :type "Vector Structure") (HitNormal :type "Vector Structure") (NormalImpulse :type "Vector Structure") (Hit :type "HitResult Structure (by ref)"))
  (bind _returnvalue (- (`self.health`) 10.0))
  (cast `/Game/BluePrints/PlayerProjectile` Other)
  (if (<= _returnvalue 0.0)
    (`self.K2_DestroyActor`)
    (else
      (set `self.health` _returnvalue))))

(fn `UserConstructionScript`)