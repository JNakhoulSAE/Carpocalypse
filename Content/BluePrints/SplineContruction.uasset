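; Blueprint that merges the splines of all actors tagged "Track" into one combined spline.
; Its construction script gathers each tagged actor's spline component, then copies every point's local-space transform and point type into a shared array.
; A newly added spline component receives that array, with tangents zeroed, input keys restarting per source spline and source actor transforms not applied.
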(fn `UserConstructionScript`
  ;[1 1 1] Get all spline components in scene
  (bind _outactors (`GameplayStatics.GetAllActorsWithTag` "Track"))
  (for _array_element _outactors
    (`KismetArrayLibrary.Array_Add` (`self.splinesInScene`) (`self.GetComponentByClass` _array_element "/Script/Engine.SplineComponent")))
  ;[1 1 1] Get all spline points in all of those spline components
  (for _array_element_2 (`self.splinesInScene`)
    (for _index (range (`SplineComponent.GetNumberOfSplinePoints` _array_element_2))
      (bind (_returnvalue_location _returnvalue_rotation _returnvalue_scale) (`KismetMathLibrary.BreakTransform` (`SplineComponent.GetTransformAtSplinePoint` _array_element_2 _index "Local" false)))
      (`KismetArrayLibrary.Array_Add` (`self.splinePoints`) (make `SplinePoint` (`KismetMathLibrary.Conv_IntToDouble` _index) _returnvalue_location (0.0 0.0 0.0) (0.0 0.0 0.0) _returnvalue_rotation _returnvalue_scale (`SplineComponent.GetSplinePointType` _array_element_2 _index)))))
  ;[1 1 1] Add those points to a new spline
  (bind _returnvalue (`AddComponent|NODE_AddSplineComponent-0`))
  (`SplineComponent.AddPoints` _returnvalue (`self.splinePoints`) true))