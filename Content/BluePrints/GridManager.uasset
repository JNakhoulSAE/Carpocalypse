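; Grid manager that tracks the state of track pieces being placed with the mouse.
; BeginPlay enables input and shows the cursor, and a left click marks the track placed when Placeable is set.
; Tick destroys the previous track on an update request, otherwise syncs it to the current one, and clears the current track once placed.
; Logic for detecting new tagged tracks and moving them under the cursor via line trace is disconnected.
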(event `self.ReceiveBeginPlay`
  (bind _returnvalue (`GameplayStatics.GetPlayerController` 0))
  (`self.EnableInput` _returnvalue)
  (set `PlayerController.bShowMouseCursor` true _returnvalue))

(event `Key|LeftMouseButton`
  (params (Key :type "Key Structure"))
  (:`Pressed`
    (if (`self.Placeable`)
      (set `self.TrackPlaced` true)
      (set `self.TrackGrabbed` false)
      (set `self.Placeable` false))))

(event `self.ReceiveTick`
  (params (DeltaSeconds :type "Float (single-precision)"))
  (if (`self.UpdateTrack`)
    (if (not (== (`self.PreviousTrack`) null))
      (`self.K2_DestroyActor` (`self.PreviousTrack`)))
    (set `self.UpdateTrack` false)
    (else
      (set `self.PreviousTrack` (`self.CurrentTrack`))))
  (if (`self.TrackGrabbed`)
    (set `self.TrackPlaced` false)
    (elif (`self.TrackPlaced`)
      (set `self.CurrentTrack` null))))

(fn `UserConstructionScript`)