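; BP_HealerEnemyAI is a healer enemy Blueprint that shows its health through a widget component.
; On BeginPlay it casts the widget to UIEnemyHealth, stores it and sets its MaxHealth from the enemy's Health.
; Each tick it copies the current Health into the widget, followed by a Delay with nothing after it.
; No healing or AI behavior is defined in this graph.
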(event `self.ReceiveBeginPlay`
  (bind _asuienemy_health (cast `/Game/BluePrints/UIEnemyHealth` (`WidgetComponent.GetUserWidgetObject` (`self.UIWidget`))))
  (bind _output_get (set `self.BPHealthWidget` _asuienemy_health))
  (set `/Game/BluePrints/UIEnemyHealth.maxHealth` (`self.health`) _output_get))

(event `self.ReceiveTick`
  (params (DeltaSeconds :type "Float (single-precision)"))
  (set `/Game/BluePrints/UIEnemyHealth.currentHealth` (`self.health`) (`self.BPHealthWidget`))
  (`KismetSystemLibrary.Delay` 1.0))

(fn `UserConstructionScript`)