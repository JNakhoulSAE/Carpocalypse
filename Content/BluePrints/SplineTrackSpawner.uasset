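; Spawner Blueprint that places straight or curved track piece actors on request.
; Each Tick it polls the SpawnSpline flag, then branches on SplineTrackType to pick TrackStraight or TrackCurved and a fixed rotation for that orientation or corner.
; The piece spawns at SplineTrackLocation and the flag clears, giving one piece per request; nothing in this Blueprint sets the flag, type or location.
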(event `self.ReceiveTick`
  (params (DeltaSeconds :type "Float (single-precision)"))
  (bind _splinetracklocation (`self.SplineTrackLocation`))
  (bind _splinetracklocation_2 (`self.SplineTrackLocation`))
  (bind _splinetracklocation_3 (`self.SplineTrackLocation`))
  (if (`self.SpawnSpline`)
    (if (`KismetStringLibrary.EqualEqual_StrStr` (`self.SplineTrackType`) (`self.Horizontal`))
      (`|SpawnActorFromClass` "/Game/BluePrints/TrackStraight.TrackStraight_C" (`KismetMathLibrary.MakeTransform` _splinetracklocation (struct :`Yaw` 90.0)) "Undefined" "OverrideRootScale" null null)
      (set `self.SpawnSpline` false :!label _label)
      (elif (`KismetStringLibrary.EqualEqual_StrStr` (`self.SplineTrackType`) (`self.Vertical`))
        (`|SpawnActorFromClass` "/Game/BluePrints/TrackStraight.TrackStraight_C" (`KismetMathLibrary.MakeTransform` _splinetracklocation) "Undefined" "OverrideRootScale" null null)
        (goto _label)
        (elif (`KismetStringLibrary.EqualEqual_StrStr` (`self.SplineTrackType`) (`self.TopLeft`))
          (`|SpawnActorFromClass` "/Game/BluePrints/TrackCurved.TrackCurved_C" (`KismetMathLibrary.MakeTransform` _splinetracklocation_3) "Undefined" "OverrideRootScale" null null)
          (goto _label)
          (elif (`KismetStringLibrary.EqualEqual_StrStr` (`self.SplineTrackType`) (`self.BottomLeft`))
            (`|SpawnActorFromClass` "/Game/BluePrints/TrackCurved.TrackCurved_C" (`KismetMathLibrary.MakeTransform` _splinetracklocation_3 (struct :`Yaw` 270.0)) "Undefined" "OverrideRootScale" null null)
            (goto _label)
            (elif (`KismetStringLibrary.EqualEqual_StrStr` (`self.SplineTrackType`) (`self.TopRight`))
              (`|SpawnActorFromClass` "/Game/BluePrints/TrackCurved.TrackCurved_C" (`KismetMathLibrary.MakeTransform` _splinetracklocation_2 (struct :`Yaw` 90.0)) "Undefined" "OverrideRootScale" null null)
              (goto _label)
              (elif (`KismetStringLibrary.EqualEqual_StrStr` (`self.SplineTrackType`) (`self.BottomRight`))
                (`|SpawnActorFromClass` "/Game/BluePrints/TrackCurved.TrackCurved_C" (`KismetMathLibrary.MakeTransform` _splinetracklocation_2 (struct :`Yaw` 180.0)) "Undefined" "OverrideRootScale" null null)
                (goto _label)))))))))

(fn `UserConstructionScript`)