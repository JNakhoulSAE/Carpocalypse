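; MeleeProjectile is an actor, apparently a melee attack projectile, that is held at a fixed world height every tick.
; Its Trigger overlap destroys the projectile when the other actor's display name contains "Player", and otherwise switches off StaticMesh collision.
; When an actor overlap ends, query and physics collision is restored on both StaticMesh and Cube.
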(event `self.ReceiveTick`
  (params (DeltaSeconds :type "Float (single-precision)"))
  (bind (_returnvalue_x _returnvalue_y) (`KismetMathLibrary.BreakVector` (`self.K2_GetActorLocation`)))
  (`self.K2_SetActorLocation` (`KismetMathLibrary.MakeVector` _returnvalue_x _returnvalue_y 240.0)))

(event `self.Trigger.OnComponentBeginOverlap`
  (params (OverlappedComponent :type "PrimitiveComponent Object Reference") (OtherActor :type "Actor Object Reference") (OtherComp :type "PrimitiveComponent Object Reference") (OtherBodyIndex :type Integer) (bFromSweep :type Boolean) (SweepResult :type "HitResult Structure (by ref)"))
  (if (== OverlappedComponent null)
    (if (`KismetStringLibrary.Contains` (`KismetSystemLibrary.GetDisplayName` OtherActor) (`self.Player`))
      (`self.K2_DestroyActor`)
      (else
        (`PrimitiveComponent.SetCollisionEnabled` (`self.StaticMesh`) "NoCollision")))))

(event `self.ReceiveActorEndOverlap`
  (params (OtherActor :type "Actor Object Reference"))
  (`PrimitiveComponent.SetCollisionEnabled` (`self.StaticMesh`) "QueryAndPhysics")
  (`PrimitiveComponent.SetCollisionEnabled` (`self.Cube`) "QueryAndPhysics"))

(fn `UserConstructionScript`)