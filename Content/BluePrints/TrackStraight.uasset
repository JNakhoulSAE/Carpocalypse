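; TrackStraight is a straight track piece that records the two endpoints of its Spline component when play begins.
; On BeginPlay it builds Point1 and Point2 as world-space spline points from the first two points, reading rotation, scale and input key at zero and full spline length.
; Each point uses one tangent for both arrive and leave.
; The construction script is empty, and nothing here reads the stored points.
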(event `self.ReceiveBeginPlay`
  (bind _spline (`self.Spline`))
  (bind _spline_2 (`self.Spline`))
  (bind (_location _tangent) (`SplineComponent.GetLocationAndTangentAtSplinePoint` _spline_2 1 "World"))
  (bind _returnvalue (`SplineComponent.GetSplineLength` _spline_2))
  (bind (_location_2 _tangent_2) (`SplineComponent.GetLocationAndTangentAtSplinePoint` _spline 0 "World"))
  (set `self.point1` (make `SplinePoint` (`SplineComponent.GetInputKeyAtDistanceAlongSpline` _spline 0.0) _location_2 _tangent_2 _tangent_2 (`SplineComponent.GetRotationAtDistanceAlongSpline` _spline 0.0 "World") (`SplineComponent.GetScaleAtDistanceAlongSpline` _spline 0.0) (`SplineComponent.GetSplinePointType` _spline 0)))
  (set `self.point2` (make `SplinePoint` (`SplineComponent.GetInputKeyAtDistanceAlongSpline` _spline_2 _returnvalue) _location _tangent _tangent (`SplineComponent.GetRotationAtDistanceAlongSpline` _spline_2 _returnvalue "World") (`SplineComponent.GetScaleAtDistanceAlongSpline` _spline_2 _returnvalue) (`SplineComponent.GetSplinePointType` _spline_2 1))))

(fn `UserConstructionScript`)