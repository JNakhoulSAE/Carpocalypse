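; Ranged enemy AI that wanders, approaches and shoots the player in range, and updates its health widget.
; Tick drives the states: below 30% health it seeks a healer until above 90%.
; Repeated hits from outside attack range trigger a cooldown-limited special shot, aimed using the midpoint of sampled player positions.
; An evasion trigger samples incoming projectile trajectories, tallying side and perpendicular distance to choose sidestep direction and length.
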(event `self.ReceiveBeginPlay`
  (bind (_returnvalue_x _returnvalue_y) (`KismetMathLibrary.BreakVector` (`self.K2_GetActorLocation`)))
  (bind _health (`self.Health`))
  (bind _outactors (`GameplayStatics.GetAllActorsOfClass` "/Game/BluePrints/BP_Player.BP_Player_C"))
  (set `self.Player` (`|GetArrayItem` _outactors))
  (bind _returnvalue (`EnemyHealth.SetHealth` "EType_Ranged"))
  (set `self.Health` _returnvalue)
  (`self.K2_SetActorLocation` (`KismetMathLibrary.MakeVector` _returnvalue_x _returnvalue_y 240.0))
  (set `self.CreateNewPos` true)
  (set `self.CreateNewRotation` true)
  (bind _asuienemy_health (cast `/Game/BluePrints/UIEnemyHealth` (`WidgetComponent.GetUserWidgetObject` (`self.Widget`))))
  (bind _output_get (set `self.BP HealthWidget` _asuienemy_health))
  (set `/Game/BluePrints/UIEnemyHealth.maxHealth` _health _output_get)
  (set `self.MaxHP` _health)
  (set `self.NormalState` true)
  (set `self.StartTimer` true)
  (set `self.SetStartPos` true))

(event `self.ReceiveHit`
  (params (MyComp :type "PrimitiveComponent Object Reference") (Other :type "Actor Object Reference") (OtherComp :type "PrimitiveComponent Object Reference") (bSelfMoved :type Boolean) (HitLocation :type "Vector Structure") (HitNormal :type "Vector Structure") (NormalImpulse :type "Vector Structure") (Hit :type "HitResult Structure (by ref)"))
  (bind _returnvalue (- (`self.Health`) 10.0))
  (cast `/Game/BluePrints/PlayerProjectile` Other)
  (`GameplayStatics.PlaySound2D` null)
  (if (<= _returnvalue 0.0)
    (`self.K2_DestroyActor`)
    (else
      (set `self.Health` _returnvalue)
      (`/Engine/EditorBlueprintResources/StandardMacros.IncrementInt` (`self.HitCount`)))))

(event `self.ReceiveTick`
  (params (DeltaSeconds :type "Float (single-precision)"))
  (bind (_returnvalue_x _returnvalue_y) (`KismetMathLibrary.BreakVector` (`self.K2_GetActorLocation`)))
  (bind (_returnvalue_roll _returnvalue_pitch _returnvalue_yaw) (`KismetMathLibrary.BreakRotator` (`self.K2_GetActorRotation`)))
  (bind _rangedenemy (`self.RangedEnemy`))
  (bind _rangedenemy_2 (`self.RangedEnemy`))
  (bind _currentclosesthealer (`self.CurrentClosestHealer`))
  (bind _rightresult (`self.RightResult`))
  (bind (_dodgestartpos_x _dodgestartpos_y) (`KismetMathLibrary.BreakVector` (`self.DodgeStartPos`)))
  (bind _leftresult (`self.LeftResult`))
  (bind _rangedenemy_3 (`self.RangedEnemy`))
  (bind _player (`self.Player`))
  (bind (_returnvalue_x_2 _returnvalue_y_2 _returnvalue_z) (`KismetMathLibrary.BreakVector` (`SceneComponent.K2_GetComponentLocation` (`self.RangedEnemy`))))
  (bind _returnvalue_location (`KismetMathLibrary.BreakTransform` (`SceneComponent.K2_GetComponentToWorld` (`self.RangedEnemy`))))
  (bind _returnvalue (`SceneComponent.K2_GetComponentLocation` _rangedenemy))
  (bind _returnvalue_location_2 (`KismetMathLibrary.BreakTransform` (`SceneComponent.K2_GetComponentToWorld` (`self.RangedEnemy`))))
  (bind (_returnvalue_x_3 _returnvalue_y_3) (`KismetMathLibrary.BreakVector` (`self.K2_GetActorLocation` (`self.Player`))))
  (bind (_returnvalue_roll_2 _returnvalue_pitch_2 _returnvalue_yaw_2) (`KismetMathLibrary.BreakRotator` (`KismetMathLibrary.FindLookAtRotation` (`SceneComponent.K2_GetComponentLocation` _rangedenemy_3) (`self.K2_GetActorLocation` (`self.Player`)))))
  (bind (_returnvalue_roll_3 _returnvalue_pitch_3 _returnvalue_yaw_3) (`KismetMathLibrary.BreakRotator` (`KismetMathLibrary.FindLookAtRotation` (`SceneComponent.K2_GetComponentLocation` _rangedenemy_2) (`self.GeneratedPos`))))
  (bind (_returnvalue_roll_4 _returnvalue_pitch_4 _returnvalue_yaw_4) (`KismetMathLibrary.BreakRotator` (`KismetMathLibrary.FindLookAtRotation` _returnvalue (`self.K2_GetActorLocation` _player))))
  (bind _returnvalue_2 (`KismetMathLibrary.Sqrt` (+ (`KismetMathLibrary.Square` (- _dodgestartpos_x _returnvalue_x)) (`KismetMathLibrary.Square` (- _dodgestartpos_y _returnvalue_y)))))
  (set `self.DeltaTime` DeltaSeconds)
  (set `self.RangedAttackTimer` (+ (`self.RangedAttackTimer`) 0.01))
  (if (`self.StartTimer`)
    (`/Engine/EditorBlueprintResources/StandardMacros.IncrementFloat` (`self.ElaspedTime`)
      (:`  `
        _)))
  (set `/Game/BluePrints/UIEnemyHealth.currentHealth` (`self.Health`) (`self.BP HealthWidget`))
  (if (`self.SpecialPhase`)
    (if (`self.GenerateRotation`) :!label _label
      (if (<= (`self.RangedAttackTimer`) 0.1)
        (bind _output_get (set `self.PlayerPositionStart` (`self.K2_GetActorLocation` (`self.Player`))))
        (elif (>= (`self.RangedAttackTimer`) 4.0)
          (set `self.GenerateRotation` false)
          (bind _output_get_2 (set `self.PlayerPositionEnd` (`self.K2_GetActorLocation` (`self.Player`))))))
      (else
        (if (`self.GenerateMidPoint`)
          (bind _output_get_3 (set `self.PlayerPositionMidPoint` (`KismetMathLibrary.MakeVector` (/ (+ (.x _output_get) (.x _output_get_2)) 2.0) (/ (+ (.y _output_get) (.y _output_get_2)) 2.0) (.z _output_get_2))))
          (set `self.GenerateMidPoint` false))
        (if (`self.SetRotation`)
          (bind (_returnvalue_roll_5 _returnvalue_pitch_5 _returnvalue_yaw_5) (`KismetMathLibrary.BreakRotator` (`KismetMathLibrary.FindLookAtRotation` _output_get_3 (`self.K2_GetActorLocation` (`self.Player`)))))
          (bind (_returnvalue_roll_6 _returnvalue_pitch_6 _returnvalue_yaw_6) (`KismetMathLibrary.BreakRotator` (`KismetMathLibrary.RInterpTo` (`KismetMathLibrary.MakeRotator` 0.0 0.0 _returnvalue_yaw) (`KismetMathLibrary.MakeRotator` 0.0 0.0 _returnvalue_yaw_5) 0.0 (`self.RotationSpeed`))))
          (`SceneComponent.K2_SetWorldRotation` (`self.RangedEnemy`) (`KismetMathLibrary.MakeRotator` 0.0 0.0 _returnvalue_yaw_6) false false)
          (`KismetSystemLibrary.Delay` 0.4)
          (`|SpawnActorFromClass` "/Game/BluePrints/RangedProjectile.RangedProjectile_C" (`KismetMathLibrary.MakeTransform` (`self.K2_GetActorLocation`) (`KismetMathLibrary.MakeRotator` 0.0 0.0 _returnvalue_yaw_5)) "Undefined" "OverrideRootScale" null null)
          (`KismetSystemLibrary.Delay` 3.2)
          (set `self.HitCount` 0)
          (set `self.SpecialPhase` false)
          (set `self.SetRotation` false)
          (set `self.SpecialPhaseCD` true))
        (`KismetSystemLibrary.Delay` 8.0)
        (set `self.SetRotation` true)
        (set `self.GenerateRotation` true)
        (set `self.GenerateMidPoint` true)
        (set `self.SpecialPhaseCD` false)))
    (else
      (if (`self.SpecialPhaseCD`)
        _
        (elif (and (> (`self.GetDistanceTo` (`self.Player`)) (`self.AttackRange`)) (> (`self.HitCount`) 3))
          (set `self.RangedAttackTimer` 0.0)
          (set `self.SpecialPhase` true)
          (goto _label)
          (else
            _)))
      (if (<= (* (/ (`self.Health`) (`self.MaxHP`)) 100.0) 30.0)
        (set `self.NormalState` false)
        (bind _outactors (`GameplayStatics.GetAllActorsOfClass` "/Game/BluePrints/BP_Healer.BP_Healer_C" :!label _label_2))
        (if (not (!= (`self.Closest Healer`) null))
          (bind _output_get_4 (set `self.NearbyEnemies` _outactors))
          (for _array_element _output_get_4
            (if (`KismetStringLibrary.Contains` (`KismetSystemLibrary.GetDisplayName` _array_element) (`self.HealerEnemy`))
              (if (!= (`self.Closest Healer`) null)
                (bind _output_get_5 (set `self.TempHealer` _array_element))
                (if (< (`self.GetDistanceTo` _output_get_5) (`self.GetDistanceTo` null))
                  (set `self.Closest Healer` (`self.TempHealer`)))
                (else
                  (set `self.Closest Healer` _array_element)))))
          (set `self.CurrentClosestHealer` (`self.Closest Healer`))
          (set `self.Closest Healer` (`self.Null`)))
        (if (not (<= (`self.GetDistanceTo` _currentclosesthealer) (`self.ProximityFromHealer`)))
          (`self.K2_SetActorLocation` (`KismetMathLibrary.VInterpTo` (`self.K2_GetActorLocation`) (`self.K2_GetActorLocation` _currentclosesthealer) (`self.DeltaTime`) (`self.Speed`))))
        (if (> (* (/ (`self.Health`) (`self.MaxHP`)) 100.0) 90.0)
          (set `self.NormalState` true)
          (elif (<= (`self.GetDistanceTo` null) (`self.AttackRange`))
            (`SceneComponent.K2_SetWorldRotation` _rangedenemy_3 (`KismetMathLibrary.MakeRotator` 0.0 0.0 _returnvalue_yaw_2) false false)))
        (else
          ;[1 1 1] Checking if the player is in the attack range
          (if (`self.NormalState`)
            (if (`self.Dodge`)
              (if (`self.SetStartPos`)
                (set `self.DodgeStartPos` (`self.K2_GetActorLocation`))
                (set `self.SetStartPos` false))
              (if (`KismetStringLibrary.EqualEqual_StrStr` (`self.DodgeDirection`) "Left")
                (if (< _leftresult 1.0)
                  (set `self.LeftResult` 1.0))
                (if (>= _returnvalue_2 (/ 400.0 _leftresult))
                  (set `self.Dodge` false :!label _label_3)
                  (set `self.ElaspedTime` 0.0)
                  (set `self.LeftValues` 0)
                  (set `self.RightValues` 0)
                  (set `self.LeftValuesAvg` 0.0)
                  (set `self.RightValuesAvg` 0.0)
                  (set `self.LeftResult` 0.0)
                  (set `self.RightResult` 0.0)
                  (set `self.StartTimer` true)
                  (else
                    (`self.K2_SetActorLocation` (- (`self.K2_GetActorLocation`) (* (`self.GetActorRightVector`) 6.0)))))
                (else
                  (if (< _rightresult 1.0)
                    (set `self.RightResult` 1.0))
                  (if (>= _returnvalue_2 (/ 400.0 _rightresult))
                    (goto _label_3)
                    (else
                      (`self.K2_SetActorLocation` (+ (`self.K2_GetActorLocation`) (* (`self.GetActorRightVector`) 6.0)))))))
              (elif (<= (`self.GetDistanceTo` _player) (`self.AttackRange`))
                (set `self.HitCount` 0)
                ;[1 1 1] Setting rotation when in attack range
                (`SceneComponent.K2_SetWorldRotation` _rangedenemy (`KismetMathLibrary.MakeRotator` 0.0 0.0 _returnvalue_yaw_4) false false)
                (if (not (<= (`self.GetDistanceTo` (`self.Player`)) (`self.ProximityFromPlayer`)))
                  (`self.K2_SetActorLocation` (`KismetMathLibrary.VInterpTo` (`self.K2_GetActorLocation`) (`KismetMathLibrary.MakeVector` _returnvalue_x_3 _returnvalue_y_3 240.0) (`self.DeltaTime`) (`self.Speed`))))
                (`KismetSystemLibrary.Delay` 0.4)
                (`|SpawnActorFromClass` "/Game/BluePrints/RangedProjectile.RangedProjectile_C" (`KismetMathLibrary.MakeTransform` _returnvalue (`KismetMathLibrary.MakeRotator` 0.0 0.0 _returnvalue_yaw_4)) "Undefined" "OverrideRootScale" null null)
                (elif (`self.CreateNewPos`)
                  ;[1 1 1] Plus or Minus Generator
                  (if (`KismetMathLibrary.RandomBool`)
                    (set `self.xSign` 1)
                    (else
                      (set `self.xSign` -1)))
                  (if (`KismetMathLibrary.RandomBool`)
                    (set `self.ySign` 1)
                    (else
                      (set `self.ySign` -1)))
                  ;[1 1 1] Calculating a random position to move to within a certain range
                  (bind _output_get_6 (set `self.GeneratedPos` (`KismetMathLibrary.MakeVector` (+ (* (`KismetMathLibrary.RandomFloatInRange` 150.0 350.0) (`KismetMathLibrary.Conv_IntToDouble` (`self.xSign`))) _returnvalue_x_2) (+ _returnvalue_y_2 (* (`KismetMathLibrary.Conv_IntToDouble` (`self.ySign`)) (`KismetMathLibrary.RandomFloatInRange` 150.0 350.0))) _returnvalue_z)))
                  ;[1 1 1] Generate a new pos if close
                  (if (== _output_get_6 _returnvalue_location_2 :`ErrorTolerance` 10.0)
                    (`KismetSystemLibrary.Delay` 0.1 :!label _label_4)
                    (set `self.CreateNewPos` true)
                    (set `self.CreateNewRotation` true)
                    (else
                      (set `self.CreateNewPos` false :!label _label_5)
                      (if (`self.CreateNewRotation`)
                        ;[1 1 1] Setting rotation to the generated position
                        (`SceneComponent.K2_SetWorldRotation` _rangedenemy_2 (`KismetMathLibrary.MakeRotator` 0.0 0.0 _returnvalue_yaw_3) false false)
                        (set `self.CreateNewRotation` false))
                      ;[1 1 1] Moving the enemy to its generated position
                      (`self.K2_SetActorLocation` (`KismetMathLibrary.VInterpTo` (`self.K2_GetActorLocation`) (`self.GeneratedPos`) (`self.DeltaTime`) (`self.Speed`)))))
                  (else
                    ;[1 1 1] If rotation is already generated
                    (if (== (`self.GeneratedPos`) _returnvalue_location :`ErrorTolerance` 10.0)
                      (goto _label_4)
                      (else
                        (goto _label_5)))))))
            (else
              (goto _label_2))))))))

(event `self.EvasionTrigger.OnComponentBeginOverlap`
  (params (OverlappedComponent :type "PrimitiveComponent Object Reference") (OtherActor :type "Actor Object Reference") (OtherComp :type "PrimitiveComponent Object Reference") (OtherBodyIndex :type Integer) (bFromSweep :type Boolean) (SweepResult :type "HitResult Structure (by ref)"))
  (bind (_firstvector_x _firstvector_y) (`KismetMathLibrary.BreakVector` (`self.FirstVector`)))
  (bind (_secondvector_x _secondvector_y) (`KismetMathLibrary.BreakVector` (`self.SecondVector`)))
  (bind (_firstvector_x_2 _firstvector_y_2) (`KismetMathLibrary.BreakVector` (`self.FirstVector`)))
  (bind (_rangedenemypt_x _rangedenemypt_y) (`KismetMathLibrary.BreakVector` (`self.RangedEnemyPt`)))
  (bind (_firstvector_x_3 _firstvector_y_3) (`KismetMathLibrary.BreakVector` (`self.FirstVector`)))
  (bind (_secondvector_x_2 _secondvector_y_2) (`KismetMathLibrary.BreakVector` (`self.SecondVector`)))
  (bind _returnvalue (`self.K2_GetActorLocation` (`self.CurrentProjectile`)))
  (bind _returnvalue_2 (- _secondvector_x_2 _firstvector_x_3))
  (bind _returnvalue_3 (- _firstvector_y_3 _secondvector_y_2))
  (bind (_returnvalue_x _returnvalue_y) (`KismetMathLibrary.BreakVector` (`SceneComponent.K2_GetComponentLocation` (`self.RangedEnemy`))))
  (bind (_returnvalue_x_2 _returnvalue_y_2) (`KismetMathLibrary.BreakVector` (`SceneComponent.K2_GetComponentLocation` (`self.RangedEnemy`))))
  (bind _returnvalue_4 (`KismetSystemLibrary.GetDisplayName` (`self.CurrentProjectile`)))
  (if (not (`self.Dodge`))
    (set `self.CurrentProjectile` OtherActor)
    (if (`KismetStringLibrary.Contains` _returnvalue_4 (`self.PlayerProjectile`))
      (for _array_element (`self.PlayerProjectiles`)
        (if (`KismetStringLibrary.EqualEqual_StrStr` _array_element _returnvalue_4)
          (set `self.Error` true)
          (break)
          (else
            (set `self.Error` false))))
      (if (not (`self.Error`))
        (`KismetArrayLibrary.Array_Add` (`self.PlayerProjectiles`) _returnvalue_4)
        (set `self.FirstVector` _returnvalue)
        (`KismetSystemLibrary.Delay` 0.05)
        (set `self.SecondVector` _returnvalue)
        (set `self.PerpendicularDist` (/ (`KismetMathLibrary.Abs` (+ (+ (* _returnvalue_x_2 _returnvalue_3) (* _returnvalue_y_2 _returnvalue_2)) (+ (* (- _firstvector_x _secondvector_x) _firstvector_y) (* (- _secondvector_y _firstvector_y) _firstvector_x)))) (+ (`KismetMathLibrary.Square` _returnvalue_3) (`KismetMathLibrary.Square` _returnvalue_2))))
        (set `self.RangedEnemyPt` (+ (`self.K2_GetActorLocation`) (* (`self.GetActorForwardVector`) 4.0)))
        (if (<= (- (* (- _returnvalue_x _rangedenemypt_x) (- _firstvector_y_2 _rangedenemypt_y)) (* (- _returnvalue_y _rangedenemypt_y) (- _firstvector_x_2 _rangedenemypt_x))) 0.0)
          (`/Engine/EditorBlueprintResources/StandardMacros.IncrementInt` (`self.LeftValues`)
            (:`  `
              (set `self.LeftValuesAvg` (+ (`self.LeftValuesAvg`) (`self.PerpendicularDist`)))))
          (else
            (`/Engine/EditorBlueprintResources/StandardMacros.IncrementInt` (`self.RightValues`)
              (:`  `
                (set `self.RightValuesAvg` (+ (`self.RightValuesAvg`) (`self.PerpendicularDist`)))))))
        (if (>= (`self.ElaspedTime`) 300.0)
          (set `self.StartTimer` false)
          (if (> (`self.LeftValues`) (`self.RightValues`))
            (set `self.LeftResult` (/ (`self.LeftValuesAvg`) (`KismetMathLibrary.Conv_IntToDouble` (`self.LeftValues`))) :!label _label_6)
            (set `self.DodgeDirection` "Left")
            (else
              (if true
                _
                (elif (== (`KismetMathLibrary.RandomIntegerInRange` 1 2) 1)
                  (goto _label_6)
                  (else
                    _)))
              (set `self.RightResult` (/ (`self.RightValuesAvg`) (`KismetMathLibrary.Conv_IntToDouble` (`self.RightValues`))))
              (set `self.DodgeDirection` "Right")))
          (set `self.Dodge` true))))))

(fn `UserConstructionScript`)