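; WinLoseConditions is an actor that shows the win or lose screen.
; It creates both widgets on BeginPlay, then polls on Tick while TotalEnemies is above zero.
; Lose takes priority, showing LoseUI and playing the game-over sound, with the GameOver flag cleared to prevent repeats.
; Otherwise WinUI appears once EnemiesKilled reaches TotalEnemies; both AddToViewport calls repeat each tick while their condition holds.
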(event `self.ReceiveBeginPlay`
  (bind _returnvalue (`|CreateWidget` "/Game/BluePrints/LoseUI.LoseUI_C"))
  (set `self.LoseUIDisplay` _returnvalue)
  (bind _returnvalue_2 (`|CreateWidget` "/Game/BluePrints/WinUI.WinUI_C"))
  (set `self.WinUIDisplay` _returnvalue_2))

(event `self.ReceiveTick`
  (params (DeltaSeconds :type "Float (single-precision)"))
  (if (> (`self.TotalEnemies`) 0)
    (if (`self.Lose`)
      (`UserWidget.AddToViewport` (`self.LoseUIDisplay`) 0)
      (if (`self.GameOver`)
        (`GameplayStatics.PlaySound2D` "/Game/Sounds/Game_Over_Sound.Game_Over_Sound")
        (set `self.GameOver` false))
      (elif (>= (`self.EnemiesKilled`) (`self.TotalEnemies`))
        (`UserWidget.AddToViewport` (`self.WinUIDisplay`) 0)))))

(fn `UserConstructionScript`)