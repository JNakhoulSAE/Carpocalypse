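; Placeable bottom-left rail piece that registers the "BL_Track" tag with the level's GridManager on BeginPlay.
; Each Tick it counts overlapping TileTrigger components and marks the grid Placeable only when exactly one overlaps.
; Once the GridManager reports the track placed, it snaps to that TrackTile's location and flags the tile's DestroyTrigger.
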(event `self.ReceiveBeginPlay`
  (bind _outactors (`GameplayStatics.GetAllActorsOfClass` "/Game/BluePrints/GridManager.GridManager_C"))
  (bind _output_get (set `self.Grid` (`|GetArrayItem` _outactors)))
  (bind _asgrid_manager (cast `/Game/BluePrints/GridManager` _output_get))
  (bind _output_get_2 (set `self.GridAccess` _asgrid_manager))
  (set `/Game/BluePrints/GridManager.TrackTag` "BL_Track" _output_get_2))

(event `self.ReceiveActorBeginOverlap`
  (params (OtherActor :type "Actor Object Reference"))
  (set `self.Position` (`self.K2_GetActorLocation` OtherActor)))

(event `self.ReceiveTick`
  (params (DeltaSeconds :type "Float (single-precision)"))
  (bind _gridaccess (`self.GridAccess`))
  (set `self.OverlappingComponents` 0)
  (for _array_element (`PrimitiveComponent.GetOverlappingComponents` (`self.Trigger`))
    (if (`KismetStringLibrary.Contains` (`KismetSystemLibrary.GetDisplayName` _array_element) (`self.TileTrigger`))
      (`/Engine/EditorBlueprintResources/StandardMacros.IncrementInt` (`self.OverlappingComponents`))))
  (if (== (`self.OverlappingComponents`) 1)
    (set `self.TrackActor` (`|GetArrayItem` (`PrimitiveComponent.GetOverlappingActors` (`self.Trigger`) "/Game/BluePrints/TrackTile.TrackTile_C")))
    (set `/Game/BluePrints/GridManager.Placeable` true _gridaccess)
    (if (`/Game/BluePrints/GridManager.TrackPlaced` (`self.GridAccess`))
      (bind _output_get (set `self.Position` (`self.K2_GetActorLocation` (`self.TrackActor`))))
      (`self.K2_SetActorLocation` _output_get)
      (bind _astrack_tile (cast `/Game/BluePrints/TrackTile` (`self.TrackActor`)))
      (set `/Game/BluePrints/TrackTile.DestroyTrigger` true _astrack_tile))
    (else
      (set `/Game/BluePrints/GridManager.Placeable` false _gridaccess))))

(fn `UserConstructionScript`)