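; BP_Melee is a melee enemy that wanders, chases and rams the player, and loses health to player projectiles until destroyed.
; Tick drives a boolean state machine, moving it with VInterpTo through ram, back-off and cooldown phases.
; Outside a ram, low health sends it to the closest overlapping healer, while a weakened ranged ally prompts a defensive move computed from ally and player positions.
; A widget mirrors its health.
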(event `self.ReceiveBeginPlay`
  (bind (_returnvalue_x _returnvalue_y) (`KismetMathLibrary.BreakVector` (`self.K2_GetActorLocation`)))
  (bind _health (`self.Health`))
  (bind _outactors (`GameplayStatics.GetAllActorsOfClass` "/Game/BluePrints/BP_Player.BP_Player_C"))
  (set `self.Player` (`|GetArrayItem` _outactors))
  (bind _outactors_2 (`GameplayStatics.GetAllActorsOfClass` "/Game/BluePrints/BP_Ranged.BP_Ranged_C"))
  (set `self.RangedEnemy` (`|GetArrayItem` _outactors_2))
  (bind _returnvalue (`EnemyHealth.SetHealth` "EType_Melee"))
  (set `self.Health` _returnvalue)
  (`self.K2_SetActorLocation` (`KismetMathLibrary.MakeVector` _returnvalue_x _returnvalue_y 240.0))
  (set `self.CreateNewPos` true)
  (set `self.CreateNewRotation` true)
  (bind _asuienemy_health (cast `/Game/BluePrints/UIEnemyHealth` (`WidgetComponent.GetUserWidgetObject` (`self.Widget`))))
  (bind _output_get (set `self.BP HealthWidget` _asuienemy_health))
  (set `/Game/BluePrints/UIEnemyHealth.maxHealth` _health _output_get)
  (set `self.MaxHP` _health)
  (set `self.AttackComplete` true)
  (set `self.Fight` true)
  (set `self.Defend` true)
  (set `self.RamState` false)
  (set `self.RetrieveState` false)
  (set `self.RefreshStates` true))

(event `self.ReceiveHit`
  (params (MyComp :type "PrimitiveComponent Object Reference") (Other :type "Actor Object Reference") (OtherComp :type "PrimitiveComponent Object Reference") (bSelfMoved :type Boolean) (HitLocation :type "Vector Structure") (HitNormal :type "Vector Structure") (NormalImpulse :type "Vector Structure") (Hit :type "HitResult Structure (by ref)"))
  (bind _returnvalue (- (`self.Health`) 24.0))
  (cast `/Game/BluePrints/PlayerProjectile` Other)
  (if (<= _returnvalue 0.0)
    (`self.K2_DestroyActor`)
    (else
      (set `self.Health` _returnvalue))))

(event `self.ReceiveTick`
  (params (DeltaSeconds :type "Float (single-precision)"))
  (bind _currentclosesthealer (`self.CurrentClosestHealer`))
  (bind _melee_enemy (`self.Melee Enemy`))
  (bind _melee_enemy_2 (`self.Melee Enemy`))
  (bind _melee_enemy_3 (`self.Melee Enemy`))
  (bind _rangedenemy (`self.RangedEnemy`))
  (bind _player (`self.Player`))
  (bind (_returnvalue_x _returnvalue_y _returnvalue_z) (`KismetMathLibrary.BreakVector` (`SceneComponent.K2_GetComponentLocation` (`self.Melee Enemy`))))
  (bind _returnvalue_location (`KismetMathLibrary.BreakTransform` (`SceneComponent.K2_GetComponentToWorld` (`self.Melee Enemy`))))
  (bind (_returnvalue_x_2 _returnvalue_y_2) (`KismetMathLibrary.BreakVector` (`self.K2_GetActorLocation` (`self.Player`))))
  (bind (_returnvalue_x_3 _returnvalue_y_3) (`KismetMathLibrary.BreakVector` (`self.K2_GetActorLocation` (`self.Player`))))
  (bind _returnvalue_location_2 (`KismetMathLibrary.BreakTransform` (`SceneComponent.K2_GetComponentToWorld` (`self.Melee Enemy`))))
  (bind _returnvalue (`self.GetDistanceTo` (`self.Player`)))
  (bind (_returnvalue_x_4 _returnvalue_y_4) (`KismetMathLibrary.BreakVector` (`self.K2_GetActorLocation` (`self.RangedEnemy`))))
  (bind (_returnvalue_x_5 _returnvalue_y_5) (`KismetMathLibrary.BreakVector` (`self.K2_GetActorLocation` (`self.Player`))))
  (bind (_returnvalue_roll _returnvalue_pitch _returnvalue_yaw) (`KismetMathLibrary.BreakRotator` (`KismetMathLibrary.FindLookAtRotation` (`SceneComponent.K2_GetComponentLocation` _melee_enemy) (`self.K2_GetActorLocation` _player))))
  (bind (_returnvalue_roll_2 _returnvalue_pitch_2 _returnvalue_yaw_2) (`KismetMathLibrary.BreakRotator` (`KismetMathLibrary.FindLookAtRotation` (`SceneComponent.K2_GetComponentLocation` _melee_enemy_2) (`self.K2_GetActorLocation` (`self.Player`)))))
  (bind (_returnvalue_roll_3 _returnvalue_pitch_3 _returnvalue_yaw_3) (`KismetMathLibrary.BreakRotator` (`KismetMathLibrary.FindLookAtRotation` (`SceneComponent.K2_GetComponentLocation` _melee_enemy_3) (`self.GeneratedPos`))))
  (bind _returnvalue_2 (* (/ (`self.Health`) (`self.MaxHP`)) 100.0))
  (set `self.DeltaTime` DeltaSeconds)
  (set `/Game/BluePrints/UIEnemyHealth.currentHealth` (`self.Health`) (`self.BP HealthWidget`))
  (if (`self.RamState`)
    ;[1 1 1] Checking if the player is in the attack range
    (if (<= (`self.GetDistanceTo` _player) (`self.FollowRange`)) :!label _label
      ;[1 1 1] Setting rotation when in follow range
      (`SceneComponent.K2_SetWorldRotation` _melee_enemy (`KismetMathLibrary.MakeRotator` 0.0 0.0 _returnvalue_yaw) false false :!label _label_2)
      (if (<= (`self.GetDistanceTo` (`self.Player`)) (`self.AttackRange`))
        (if (`self.RefreshStates`)
          (set `self.RamState` true)
          (set `self.RetrieveState` true)
          (set `self.RefreshStates` false)
          (else
            (if (`self.RamState`) :!label _label_3
              (if (<= (`self.GetDistanceTo` (`self.Player`)) (`self.ProximityFromPlayer`))
                (set `self.RamState` false)
                (set `self.RetrieveDistance` (`KismetMathLibrary.RandomFloatInRange` 420.0 520.0))
                (else
                  (`self.K2_SetActorLocation` (`KismetMathLibrary.VInterpTo` (`self.K2_GetActorLocation`) (`KismetMathLibrary.MakeVector` _returnvalue_x_3 _returnvalue_y_3 240.0) (`self.DeltaTime`) (`self.RamSpeed`)))))
              (elif (`self.RetrieveState`)
                (`self.K2_SetActorLocation` (- (`self.K2_GetActorLocation`) (* (`self.GetActorForwardVector`) 4.0)))
                (`KismetSystemLibrary.PrintString` (`KismetStringLibrary.Conv_DoubleToString` _returnvalue))
                (if (>= _returnvalue (`self.RetrieveDistance`))
                  (set `self.RetrieveState` false))
                (else
                  (set `self.AttackComplete` true)
                  (`KismetSystemLibrary.Delay` (`KismetMathLibrary.RandomFloatInRange` 4.0 4.5))
                  (set `self.RefreshStates` true))))))
        (elif (`self.RetrieveState`)
          (goto _label_3)
          (else
            (`self.K2_SetActorLocation` (`KismetMathLibrary.VInterpTo` (`self.K2_GetActorLocation`) (`KismetMathLibrary.MakeVector` _returnvalue_x_2 _returnvalue_y_2 240.0) (`self.DeltaTime`) (`self.Speed`)))
            (goto _label_3))))
      (elif (`self.AttackComplete`)
        (if (`self.CreateNewPos`)
          ;[1 1 1] Plus or Minus Generator
          (if (`KismetMathLibrary.RandomBool`)
            (set `self.xSign` 1)
            (else
              (set `self.xSign` -1)))
          (if (`KismetMathLibrary.RandomBool`)
            (set `self.ySign` 1)
            (else
              (set `self.ySign` -1)))
          ;[1 1 1] Calculating a random position to move to within a certain range
          (bind _output_get (set `self.GeneratedPos` (`KismetMathLibrary.MakeVector` (+ (* (`KismetMathLibrary.RandomFloatInRange` 150.0 350.0) (`KismetMathLibrary.Conv_IntToDouble` (`self.xSign`))) _returnvalue_x) (+ _returnvalue_y (* (`KismetMathLibrary.Conv_IntToDouble` (`self.ySign`)) (`KismetMathLibrary.RandomFloatInRange` 200.0 450.0))) _returnvalue_z)))
          ;[1 1 1] Generate a new pos if close
          (if (== _output_get _returnvalue_location_2 :`ErrorTolerance` 10.0)
            (`KismetSystemLibrary.Delay` 0.1 :!label _label_4)
            (set `self.CreateNewPos` true)
            (set `self.CreateNewRotation` true)
            (else
              (set `self.CreateNewPos` false :!label _label_5)
              (if (`self.CreateNewRotation`)
                ;[1 1 1] Setting rotation to the generated position
                (`SceneComponent.K2_SetWorldRotation` _melee_enemy_3 (`KismetMathLibrary.MakeRotator` 0.0 0.0 _returnvalue_yaw_3) false false)
                (set `self.CreateNewRotation` false))
              ;[1 1 1] Moving the enemy to its generated position
              (`self.K2_SetActorLocation` (`KismetMathLibrary.VInterpTo` (`self.K2_GetActorLocation`) (`self.GeneratedPos`) (`self.DeltaTime`) (`self.Speed`)))))
          (else
            ;[1 1 1] If rotation is already generated
            (if (== (`self.GeneratedPos`) _returnvalue_location :`ErrorTolerance` 10.0)
              (goto _label_4)
              (else
                (goto _label_5)))))
        (else
          (goto _label_2))))
    (elif (<= _returnvalue_2 50.0)
      (set `self.Fight` false)
      ;[1 1 1] Finding Closest Healer
      (if (not (!= (`self.ClosestHealer`) null)) :!label _label_6
        (bind _output_get_2 (set `self.NearbyEnemies` (`PrimitiveComponent.GetOverlappingActors` (`self.MeleeTrigger`) null)))
        (for _array_element _output_get_2
          (if (`KismetStringLibrary.Contains` (`KismetSystemLibrary.GetDisplayName` _array_element) (`self.HealerEnemy`))
            (if (!= (`self.ClosestHealer`) null)
              (bind _output_get_3 (set `self.TempHealer` _array_element))
              (if (< (`self.GetDistanceTo` _output_get_3) (`self.GetDistanceTo` (stale _output_get_4)))
                (set `self.ClosestHealer` (`self.TempHealer`)))
              (else
                (bind _output_get_4 (set `self.ClosestHealer` _array_element))))))
        (set `self.CurrentClosestHealer` (`self.ClosestHealer`))
        (set `self.ClosestHealer` (`self.Null`)))
      (if (not (<= (`self.GetDistanceTo` _currentclosesthealer) (`self.ProximityFromHealer`)))
        (`self.K2_SetActorLocation` (`KismetMathLibrary.VInterpTo` (`self.K2_GetActorLocation`) (`self.K2_GetActorLocation` _currentclosesthealer) (`self.DeltaTime`) (`self.Speed`))))
      (if (not (< (* (/ (`self.Health`) (`self.MaxHP`)) 100.0) 75.0))
        (if (not (`self.ThresholdGenerated`))
          (set `self.RNG Int` (`KismetMathLibrary.RandomIntegerInRange` 1 10))
          (set `self.ThresholdGenerated` true))
        (if (>= (* (/ (`self.Health`) (`self.MaxHP`)) 100.0) 75.0)
          (if (<= (`self.RNG Int`) 3)
            (`KismetSystemLibrary.Delay` 2.25)
            (set `self.Fight` true)
            (elif (== (> (`self.RNG Int`) 3) (<= (`self.RNG Int`) 6))
              (`KismetSystemLibrary.Delay` 5.0)
              (set `self.Fight` true)
              (else
                (`KismetSystemLibrary.Delay` 6.5)
                (set `self.Fight` true))))))
      (elif (and (> _returnvalue_2 74.0) (<= (* (/ (`/Game/BluePrints/BP_Ranged.Health` _rangedenemy) (`/Game/BluePrints/BP_Ranged.MaxHP` _rangedenemy)) 100.0) 45.0))
        (set `self.Fight` false)
        ;[1 1 1] Defence Mechanism
        (set `self.DistOverDist` (/ (`KismetMathLibrary.RandomFloatInRange` 150.0 300.0) (`self.GetDistanceTo` (`self.RangedEnemy`) (`self.Player`))))
        (set `self.xCoordDef` (* (- 1.0 (`self.DistOverDist`)) (+ _returnvalue_x_5 _returnvalue_x_4)))
        (set `self.yCoordDef` (* (- 1.0 (`self.DistOverDist`)) (+ _returnvalue_y_5 _returnvalue_y_4)))
        (`self.K2_SetActorLocation` (`KismetMathLibrary.VInterpTo` (`self.K2_GetActorLocation`) (`KismetMathLibrary.MakeVector` (`self.xCoordDef`) (`self.yCoordDef`) 240.0) (`self.DeltaTime`) (`self.Speed`)))
        (`SceneComponent.K2_SetWorldRotation` _melee_enemy_2 (`KismetMathLibrary.MakeRotator` 0.0 0.0 _returnvalue_yaw_2) false false)
        (`KismetSystemLibrary.Delay` (`KismetMathLibrary.RandomFloatInRange` 1.0 2.25))
        (set `self.Fight` true)
        (elif (`self.Fight`)
          (goto _label)
          (else
            (goto _label_6)))))))

(fn `UserConstructionScript`)