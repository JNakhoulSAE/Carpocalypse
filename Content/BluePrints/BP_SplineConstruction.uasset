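; Actor that builds one spline at runtime from placed TrackStraight and TrackCurved pieces, starting at its own location.
; SpherePoint2 follows the spline end on Tick; overlaps at BeginPlay or on begin-overlap feed GetPointToAdd.
; That function identifies triggers by name, returning the piece's opposite point, tangents negated for reversed entry; the piece is then destroyed.
; Returning near the start marks completion, though SetClosedLoop receives false.
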(event `self.ReceiveBeginPlay`
  (bind _overlappingcomponents (`self.overlappingComponents`))
  (if (not (`self.splineFinished`)) :!label _label
    (set `self.overlappingComponents` (`PrimitiveComponent.GetOverlappingComponents` (`self.spherePoint2`)))
    (if (`KismetArrayLibrary.Array_IsValidIndex` _overlappingcomponents)
      (for _array_element _overlappingcomponents
        (bind (_pointtoadd _triggerwasvalid) (`self.GetPointToAdd` _array_element)) ; Custom script
        (if _triggerwasvalid
          (bind (_inputkey _position _arrivetangent _leavetangent) (break `SplinePoint` _pointtoadd))
          ;[1 1 1] Add point and set tangent
          (`SplineComponent.AddSplinePoint` (`self.Spline`) _position "World" true)
          (`SplineComponent.SetTangentsAtSplinePoint` (`self.Spline`) (- (`SplineComponent.GetNumberOfSplinePoints` (`self.Spline`)) 1) _arrivetangent _leavetangent "World" true)
          (set `self.endOfSpline` _position)
          (`self.K2_DestroyActor` (`ActorComponent.GetOwner` _array_element))))
      ;[1 1 1] Return to start of function if end has not been reached. If end has been reached, make the spline a loop.
      (if (== (`self.endOfSpline`) (`self.startOfSpline`) :`ErrorTolerance` 5.0)
        (`SplineComponent.SetClosedLoop` (`self.Spline`) false true)
        (set `self.splineFinished` true)
        (`KismetSystemLibrary.PrintString` "Loop detected! Spline Complete." true true (struct :`G` 0.66 :`B` 1.0 :`A` 1.0) 10.0)
        (else
          (`KismetSystemLibrary.PrintString` "Iteration complete. Spline not finished." true true (struct :`G` 0.66 :`B` 1.0 :`A` 1.0) 10.0)))
      (else
        (`KismetSystemLibrary.PrintString` "Could not detect splinePoint trigger on this iteration. Trying Again." true true (struct :`G` 0.66 :`B` 1.0 :`A` 1.0) 10.0)))))

(event `self.spherePoint2.OnComponentBeginOverlap`
  (params (OverlappedComponent :type "PrimitiveComponent Object Reference") (OtherActor :type "Actor Object Reference") (OtherComp :type "PrimitiveComponent Object Reference") (OtherBodyIndex :type Integer) (bFromSweep :type Boolean) (SweepResult :type "HitResult Structure (by ref)"))
  (goto _label))

(event `self.ReceiveTick`
  (params (DeltaSeconds :type "Float (single-precision)"))
  (if (not (`self.splineFinished`))
    (`SceneComponent.K2_SetWorldLocation` (`self.spherePoint2`) (`self.endOfSpline`) false false)
    (set `self.overlappingComponents` (`PrimitiveComponent.GetOverlappingComponents` (`self.spherePoint2`)))))

(fn `GetPointToAdd`
  (params (triggerToUse :type "PrimitiveComponent Object Reference"))
  (returns (pointToAdd :type "SplinePoint Structure") (triggerWasValid :type Boolean))
  (locals (_pointToAdd :type "SplinePoint Structure") (_triggerWasValid :type Boolean :default true))
  (bind _returnvalue (`ActorComponent.GetOwner` triggerToUse))
  (bind _returnvalue_2 (`KismetSystemLibrary.GetObjectName` triggerToUse))
  (bind _returnvalue_3 (`KismetSystemLibrary.GetDisplayName` _returnvalue))
  (if (`KismetStringLibrary.Contains` _returnvalue_2 "spherePoint1")
    (`KismetSystemLibrary.PrintString` (`KismetStringLibrary.Concat_StrStr` _returnvalue_3 " added to track.") true true (struct :`G` 0.66 :`B` 1.0 :`A` 1.0) 10.0)
    (if (`KismetStringLibrary.Contains` _returnvalue_3 "TrackStraight")
      (bind _astrack_straight (cast `/Game/BluePrints/TrackStraight` _returnvalue))
      (set `local._pointToAdd` (`/Game/BluePrints/TrackStraight.point2` _astrack_straight))
      (return (`local._pointToAdd`) (`local._triggerWasValid`))
      (elif (`KismetStringLibrary.Contains` _returnvalue_3 "TrackCurved")
        (bind _astrack_curved (cast `/Game/BluePrints/TrackCurved` _returnvalue))
        (set `local._pointToAdd` (`/Game/BluePrints/TrackCurved.point2` _astrack_curved))
        (return (`local._pointToAdd`) (`local._triggerWasValid`))))
    (elif (`KismetStringLibrary.Contains` _returnvalue_2 "spherePoint2")
      (`KismetSystemLibrary.PrintString` (`KismetStringLibrary.Concat_StrStr` _returnvalue_3 " added to track.") true true (struct :`G` 0.66 :`B` 1.0 :`A` 1.0) 10.0)
      (if (`KismetStringLibrary.Contains` _returnvalue_3 "TrackStraight")
        (bind _astrack_straight_2 (cast `/Game/BluePrints/TrackStraight` _returnvalue))
        (bind (_point1_inputkey _point1_position _point1_arrivetangent _point1_leavetangent _point1_rotation _point1_scale _point1_type) (break `SplinePoint` (`/Game/BluePrints/TrackStraight.point1` _astrack_straight_2)))
        (set `local._pointToAdd` (make `SplinePoint` _point1_inputkey _point1_position (* _point1_arrivetangent -1) (* _point1_leavetangent -1) _point1_rotation _point1_scale _point1_type))
        (return (`local._pointToAdd`) (`local._triggerWasValid`))
        (elif (`KismetStringLibrary.Contains` _returnvalue_3 "TrackCurved")
          (bind _astrack_curved_2 (cast `/Game/BluePrints/TrackCurved` _returnvalue))
          (bind (_point1_inputkey_2 _point1_position_2 _point1_arrivetangent_2 _point1_leavetangent_2 _point1_rotation_2 _point1_scale_2 _point1_type_2) (break `SplinePoint` (`/Game/BluePrints/TrackCurved.point1` _astrack_curved_2)))
          (set `local._pointToAdd` (make `SplinePoint` _point1_inputkey_2 _point1_position_2 (* _point1_arrivetangent_2 -1) (* _point1_leavetangent_2 -1) _point1_rotation_2 _point1_scale_2 _point1_type_2))
          (return (`local._pointToAdd`) (`local._triggerWasValid`))))
      (else
        (set `local._triggerWasValid` false)
        (return (`local._pointToAdd`) (`local._triggerWasValid`))))))

(fn `UserConstructionScript`
  (set `self.startOfSpline` (`self.K2_GetActorLocation`)))