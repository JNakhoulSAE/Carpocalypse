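; Placement actor for a bottom-left rail piece that follows the mouse on a tile grid until it is placed.
; On begin play it finds GridManager and SplineTrackSpawner, and overlapping a TrackTile sets the grid's shared Placeable flag.
; While Placeable is set, Tick snaps a cursor trace to 200-unit cells at fixed height.
; When it clears, the actor locks once, requests a BottomLeft spline and destroys the tile.
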(event `self.ReceiveBeginPlay`
  (bind _outactors (`GameplayStatics.GetAllActorsOfClass` "/Game/BluePrints/GridManager.GridManager_C"))
  (bind _output_get (set `self.Grid` (`|GetArrayItem` _outactors)))
  (bind _asgrid_manager (cast `/Game/BluePrints/GridManager` _output_get))
  (bind _output_get_2 (set `self.GridAccess` _asgrid_manager))
  (set `/Game/BluePrints/GridManager.TrackTag` "H_Track" _output_get_2)
  (bind _outactors_2 (`GameplayStatics.GetAllActorsOfClass` "/Game/BluePrints/SplineTrackSpawner.SplineTrackSpawner_C"))
  (bind _output_get_3 (set `self.STS` (`|GetArrayItem` _outactors_2)))
  (set `self.STSAccess` _output_get_3)
  (bind _outactors_3 (`GameplayStatics.GetAllActorsOfClass` "/Game/BluePrints/DestroyTileBP.DestroyTileBP_C"))
  (set `self.DestroyActorBPref` (`|GetArrayItem` _outactors_3))
  (`self.EnableInput` (`GameplayStatics.GetPlayerController` 0)))

(event `self.ReceiveActorBeginOverlap`
  (params (OtherActor :type "Actor Object Reference"))
  (if (`KismetStringLibrary.Contains` (`KismetSystemLibrary.GetDisplayName` OtherActor) "TrackTile")
    (set `self.TrackActor` OtherActor)
    (set `/Game/BluePrints/GridManager.Placeable` true (`self.GridAccess`))
    (set `self.Position` (`self.K2_GetActorLocation` (`self.TrackActor`)))))

(event `self.ReceiveTick`
  (params (DeltaSeconds :type "Float (single-precision)"))
  (bind _stsaccess (`self.STSAccess`))
  (bind (_worldlocation _worlddirection) (`PlayerController.DeprojectMousePositionToWorld` (`GameplayStatics.GetPlayerController` 0)))
  (if (`/Game/BluePrints/GridManager.Placeable` (`self.GridAccess`))
    (if (not (`self.thisTrackPlaced`))
      (bind _outhit (`KismetSystemLibrary.LineTraceSingle` _worldlocation (+ _worldlocation (* _worlddirection 10000.0)) "TraceTypeQuery1"))
      (bind (_bblockinghit _binitialoverlap _time _distance _location) (`GameplayStatics.BreakHitResult` _outhit))
      (bind _output_get (set `self.Position` (`KismetMathLibrary.MakeVector` (* (`KismetMathLibrary.Conv_IntToDouble` (`KismetMathLibrary.Round` (/ (.x _location) 200.0))) 200.0) (* (`KismetMathLibrary.Conv_IntToDouble` (`KismetMathLibrary.Round` (/ (.y _location) 200.0))) 200.0) 221.0)))
      (`self.K2_SetActorLocation` _output_get))
    (elif (not (`self.thisTrackPlaced`))
      (`self.K2_SetActorLocation` (`self.Position`))
      (set `/Game/BluePrints/SplineTrackSpawner.SplineTrackLocation` (`self.Position`) _stsaccess)
      (set `/Game/BluePrints/SplineTrackSpawner.SplineTrackType` "BottomLeft" _stsaccess)
      (set `/Game/BluePrints/SplineTrackSpawner.SpawnSpline` true _stsaccess)
      (set `/Game/BluePrints/GridManager.TrackPlaced` false (`self.GridAccess`))
      (set `self.thisTrackPlaced` true)
      (`self.K2_DestroyActor` (`self.TrackActor`)))))

(fn `UserConstructionScript`)