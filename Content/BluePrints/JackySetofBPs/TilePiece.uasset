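; TilePiece is a tile Blueprint that spawns a TrackActor_Jacky2 at a fixed location on BeginPlay and records spline points when a track actor touches it.
; TileTrigger overlaps match actors by "TrackActor" in the display name, then fill an empty Points array with two points derived from TileRadius and Tile's world position.
; Tick prints the overlap actor's name for debugging, and an unconnected Horizontal string comparison does nothing.
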(event `self.ReceiveBeginPlay`
  (`|SpawnActorFromClass` "/Game/BluePrints/JackySetofBPs/TrackActor_Jacky2.TrackActor_Jacky2_C" (`KismetMathLibrary.MakeTransform` (-150.0 790.0 220.0)) "AlwaysSpawn" "OverrideRootScale" null null))

(event `self.ReceiveTick`
  (params (DeltaSeconds :type "Float (single-precision)"))
  (`KismetSystemLibrary.PrintString` (`KismetSystemLibrary.GetObjectName` (stale `self.TileTrigger.OnComponentBeginOverlap` OtherActor))))

(event `self.TileTrigger.OnComponentBeginOverlap`
  (params (OverlappedComponent :type "PrimitiveComponent Object Reference") (OtherActor :type "Actor Object Reference") (OtherComp :type "PrimitiveComponent Object Reference") (OtherBodyIndex :type Integer) (bFromSweep :type Boolean) (SweepResult :type "HitResult Structure (by ref)"))
  (bind (_returnvalue_x _returnvalue_y) (`KismetMathLibrary.BreakVector` (`SceneComponent.K2_GetComponentLocation` (`self.Tile`))))
  (bind (_returnvalue_x_2 _returnvalue_y_2) (`KismetMathLibrary.BreakVector` (`SceneComponent.K2_GetComponentLocation` (`self.Tile`))))
  (if (`KismetStringLibrary.Contains` (`KismetSystemLibrary.GetDisplayName` OtherActor) (`self.TrackActor`))
    (if (not (`KismetArrayLibrary.Array_IsValidIndex` (`self.Points`)))
      (`KismetArrayLibrary.Array_Add` (`self.Points`) (make `SplinePoint` 0.0 (`KismetMathLibrary.MakeVector` (- (`self.TileRadius`) _returnvalue_x_2) _returnvalue_y_2)))
      (`KismetArrayLibrary.Array_Add` (`self.Points`) (make `SplinePoint` 0.0 (`KismetMathLibrary.MakeVector` (+ (`self.TileRadius`) _returnvalue_x) _returnvalue_y))))))

(fn `UserConstructionScript`)