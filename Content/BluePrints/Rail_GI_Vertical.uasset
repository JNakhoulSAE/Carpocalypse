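; Vertical rail placement actor that validates a spot on the track grid and requests a vertical spline track there.
; BeginPlay caches the GridManager and SplineTrackSpawner and tags the grid's track as vertical.
; Tick polls its trigger, allowing placement only when exactly one TileTrigger component, matched by name, overlaps.
; On placement it snaps to the tile at fixed height, sets the spawner's spawn flag and flags the tile's trigger for destruction.
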(event `self.ReceiveBeginPlay`
  (bind _outactors (`GameplayStatics.GetAllActorsOfClass` "/Game/BluePrints/GridManager.GridManager_C"))
  (bind _output_get (set `self.Grid` (`|GetArrayItem` _outactors)))
  (bind _asgrid_manager (cast `/Game/BluePrints/GridManager` _output_get))
  (bind _output_get_2 (set `self.GridAccess` _asgrid_manager))
  (set `/Game/BluePrints/GridManager.TrackTag` "V_Track" _output_get_2)
  (bind _outactors_2 (`GameplayStatics.GetAllActorsOfClass` "/Game/BluePrints/SplineTrackSpawner.SplineTrackSpawner_C"))
  (bind _output_get_3 (set `self.STS` (`|GetArrayItem` _outactors_2)))
  (bind _asspline_track_spawner (cast `/Game/BluePrints/SplineTrackSpawner` _output_get_3))
  (set `self.STSAccess` _asspline_track_spawner))

(event `self.ReceiveActorBeginOverlap`
  (params (OtherActor :type "Actor Object Reference"))
  (set `self.Position` (`self.K2_GetActorLocation` OtherActor)))

(event `self.ReceiveTick`
  (params (DeltaSeconds :type "Float (single-precision)"))
  (bind _stsaccess (`self.STSAccess`))
  (bind _gridaccess (`self.GridAccess`))
  (set `self.OverlappingComponents` 0)
  (for _array_element (`PrimitiveComponent.GetOverlappingComponents` (`self.Trigger`))
    (if (`KismetStringLibrary.Contains` (`KismetSystemLibrary.GetDisplayName` _array_element) (`self.TileTrigger`))
      (`/Engine/EditorBlueprintResources/StandardMacros.IncrementInt` (`self.OverlappingComponents`))))
  (if (== (`self.OverlappingComponents`) 1)
    (set `self.TrackActor` (`|GetArrayItem` (`PrimitiveComponent.GetOverlappingActors` (`self.Trigger`) "/Game/BluePrints/TrackTile.TrackTile_C")))
    (set `/Game/BluePrints/GridManager.Placeable` true _gridaccess)
    (if (`/Game/BluePrints/GridManager.TrackPlaced` (`self.GridAccess`))
      (bind _output_get (set `self.Position` (`self.K2_GetActorLocation` (`self.TrackActor`))))
      (bind _output_get_2 (set `/Game/BluePrints/SplineTrackSpawner.SplineTrackLocation` _output_get _stsaccess))
      (`self.K2_SetActorLocation` (`KismetMathLibrary.MakeVector` (.x _output_get_2) (.y _output_get_2) 240.0))
      (set `/Game/BluePrints/SplineTrackSpawner.SplineTrackType` "Vertical" _stsaccess)
      (set `/Game/BluePrints/SplineTrackSpawner.SpawnSpline` true _stsaccess)
      (bind _astrack_tile (cast `/Game/BluePrints/TrackTile` (`self.TrackActor`)))
      (set `/Game/BluePrints/TrackTile.DestroyTrigger` true _astrack_tile))
    (else
      (set `/Game/BluePrints/GridManager.Placeable` false _gridaccess))))

(fn `UserConstructionScript`)