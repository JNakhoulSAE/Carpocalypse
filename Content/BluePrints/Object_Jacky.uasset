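; Jacky is an actor that the player slides along a spline track by holding D to go forward or A to go back.
; On BeginPlay it enables input, finds the first BP_SplineConstruction_Jacky and snaps to its stored distance along that spline.
; Tick, gated by a short Delay, sets the world location from that distance, then steps it, wrapping at either end despite comments describing a stop.
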(event `self.ReceiveBeginPlay`
  (`self.EnableInput` (`GameplayStatics.GetPlayerController` 0))
  ;[1 1 1] Get Spline Track
  (bind _outactors (`GameplayStatics.GetAllActorsOfClass` "/Game/BluePrints/BP_SplineConstruction_Jacky.BP_SplineConstruction_Jacky_C"))
  (set `self.Spline_Jacky` (`|GetArrayItem` _outactors))
  (`self.K2_SetActorLocation` (`SplineComponent.GetLocationAtDistanceAlongSpline` (`/Game/BluePrints/BP_SplineConstruction_Jacky.Spline` (`self.Spline_Jacky`)) (`self.DistanceAlongSpline`) "World")))

(event `self.ReceiveTick`
  (params (DeltaSeconds :type "Float (single-precision)"))
  (bind _distancealongspline (`self.DistanceAlongSpline`))
  (bind _dpressed (`self.DPressed`))
  (bind _stepdistance (`self.StepDistance`))
  (bind _spline (`/Game/BluePrints/BP_SplineConstruction_Jacky.Spline` (`self.Spline_Jacky`)))
  (`KismetSystemLibrary.Delay` 0.01)
  (if (or _dpressed (`self.APressed`))
    ;[1 1 1] Changing distance along spline
    (`self.K2_SetActorLocation` (`SplineComponent.GetLocationAtDistanceAlongSpline` _spline _distancealongspline "World"))
    (if _dpressed
      (`/Engine/EditorBlueprintResources/StandardMacros.CompareFloat` _distancealongspline (- (`SplineComponent.GetSplineLength` _spline) _stepdistance) ; Makes sure player can't change the distance along the spline if the end has been reached
        (:`>`
          (set `self.DistanceAlongSpline` 0.0 :!label _label))
        (:`==`
          (goto _label))
        (:`<`
          _))
      (set `self.DistanceAlongSpline` (+ (`self.DistanceAlongSpline`) _stepdistance))
      (else
        (`/Engine/EditorBlueprintResources/StandardMacros.CompareFloat` _distancealongspline _stepdistance ; Makes sure player can't change the distance along the spline if the start has been reached
          (:`>`
            _)
          (:`==`
            (set `self.DistanceAlongSpline` (`SplineComponent.GetSplineLength` (`/Game/BluePrints/BP_SplineConstruction_Jacky.Spline` (`self.Spline_Jacky`))) :!label _label_2))
          (:`<`
            (goto _label_2)))
        (set `self.DistanceAlongSpline` (- (`self.DistanceAlongSpline`) _stepdistance))))))

(event `Key|A`
  (params (Key :type "Key Structure"))
  ;[1 1 1] Get key input
  (:`Pressed`
    (set `self.APressed` true))
  (:`Released`
    (set `self.APressed` false)))

(event `Key|D`
  (params (Key :type "Key Structure"))
  ;[1 1 1] Get key input
  (:`Pressed`
    (set `self.DPressed` true))
  (:`Released`
    (set `self.DPressed` false)))

(fn `UserConstructionScript`)