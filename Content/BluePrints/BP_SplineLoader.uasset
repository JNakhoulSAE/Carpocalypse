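; BP_SplineLoader spawns track piece actors on request, acting as a loader for straight and curved track segments.
; Each Tick it checks the LoadSpline flag and, when set, compares SplineType against horizontal, vertical and four corner types.
; The match spawns TrackStraight or TrackCurved at SplineLoadPosition with a fixed rotation per orientation, then clears the flag.
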(event `self.ReceiveTick`
  (params (DeltaSeconds :type "Float (single-precision)"))
  (bind _splineloadposition (`self.splineLoadPosition`))
  (bind _splineloadposition_2 (`self.splineLoadPosition`))
  (bind _splineloadposition_3 (`self.splineLoadPosition`))
  (if (`self.loadSpline`)
    (if (`KismetStringLibrary.EqualEqual_StrStr` (`self.splineType`) "Load_Horizontal")
      (`|SpawnActorFromClass` "/Game/BluePrints/TrackStraight.TrackStraight_C" (`KismetMathLibrary.MakeTransform` _splineloadposition (struct :`Yaw` 90.0)) "Undefined" "OverrideRootScale" null null)
      (set `self.loadSpline` false :!label _label)
      (elif (`KismetStringLibrary.EqualEqual_StrStr` (`self.splineType`) "Load_Vertical")
        (`|SpawnActorFromClass` "/Game/BluePrints/TrackStraight.TrackStraight_C" (`KismetMathLibrary.MakeTransform` _splineloadposition) "Undefined" "OverrideRootScale" null null)
        (goto _label)
        (elif (`KismetStringLibrary.EqualEqual_StrStr` (`self.splineType`) "Load_TL")
          (`|SpawnActorFromClass` "/Game/BluePrints/TrackCurved.TrackCurved_C" (`KismetMathLibrary.MakeTransform` _splineloadposition_3) "Undefined" "OverrideRootScale" null null)
          (goto _label)
          (elif (`KismetStringLibrary.EqualEqual_StrStr` (`self.splineType`) "Load_BL")
            (`|SpawnActorFromClass` "/Game/BluePrints/TrackCurved.TrackCurved_C" (`KismetMathLibrary.MakeTransform` _splineloadposition_3 (struct :`Yaw` 270.0)) "Undefined" "OverrideRootScale" null null)
            (goto _label)
            (elif (`KismetStringLibrary.EqualEqual_StrStr` (`self.splineType`) "Load_TR")
              (`|SpawnActorFromClass` "/Game/BluePrints/TrackCurved.TrackCurved_C" (`KismetMathLibrary.MakeTransform` _splineloadposition_2 (struct :`Yaw` 90.0)) "Undefined" "OverrideRootScale" null null)
              (goto _label)
              (elif (`KismetStringLibrary.EqualEqual_StrStr` (`self.splineType`) "Load_BR")
                (`|SpawnActorFromClass` "/Game/BluePrints/TrackCurved.TrackCurved_C" (`KismetMathLibrary.MakeTransform` _splineloadposition_2 (struct :`Yaw` 180.0)) "Undefined" "OverrideRootScale" null null)
                (goto _label)))))))))

(fn `UserConstructionScript`)