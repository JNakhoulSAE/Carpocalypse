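; EnemyMovement is a Blueprint that makes an enemy face and follow the player, moving the actor it is parented to.
; BeginPlay caches the first BP_Player found and the parent actor.
; Each Tick snaps its own rotation toward the player and, while farther away than MovementRange, moves the parent toward the player with VInterpTo at Speed.
; The move is unswept, so it ignores blocking collision and uses no pathfinding.
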(event `self.ReceiveBeginPlay`
  (bind _outactors (`GameplayStatics.GetAllActorsOfClass` "/Game/BluePrints/BP_Player.BP_Player_C"))
  (set `self.Player` (`|GetArrayItem` _outactors))
  (set `self.Parent` (`self.GetParentActor`)))

(event `self.ReceiveTick`
  (params (DeltaSeconds :type "Float (single-precision)"))
  (set `self.DeltaTime` DeltaSeconds)
  (`self.K2_SetActorRotation` (`KismetMathLibrary.FindLookAtRotation` (`self.K2_GetActorLocation`) (`self.K2_GetActorLocation` (`self.Player`))))
  (if (> (`self.GetDistanceTo` (`self.Player`)) (`self.MovementRange`))
    (`self.K2_SetActorLocation` (`self.Parent`) (`KismetMathLibrary.VInterpTo` (`self.K2_GetActorLocation` (`self.Parent`)) (`self.K2_GetActorLocation` (`self.Player`)) (`self.DeltaTime`) (`self.Speed`)) false false)))

(fn `UserConstructionScript`)