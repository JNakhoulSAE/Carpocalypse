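; Input-driven controller that moves BP_Player back and forth along a BP_Spline track with the A and D keys.
; BeginPlay caches the first spline and player found, then places the player at the current spline distance.
; Key events set held flags that Tick reads after a short Delay, repositioning the player and stepping the distance, with D taking priority.
; Comparisons against zero and spline length gate the stepping.
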(event `self.ReceiveBeginPlay`
  (`self.EnableInput` (`GameplayStatics.GetPlayerController` 0))
  ;[1 1 1] Get Spline Track
  (bind _outactors (`GameplayStatics.GetAllActorsOfClass` "/Game/BluePrints/BP_Spline.BP_Spline_C"))
  (set `self.SplineTrack` (`|GetArrayItem` _outactors))
  ;[1 1 1] Get Player
  (bind _outactors_2 (`GameplayStatics.GetAllActorsOfClass` "/Game/Blueprints/BP_Player.BP_Player_C"))
  (bind _output_get (set `self.PlayerBP` (`|GetArrayItem` _outactors_2)))
  (`self.K2_SetActorLocation` _output_get (`SplineComponent.GetLocationAtDistanceAlongSpline` (`/Game/BluePrints/BP_Spline.Spline` (`self.SplineTrack`)) (`self.DistanceAlongSpline`) "World") false false))

(event `self.ReceiveTick`
  (params (DeltaSeconds :type "Float (single-precision)"))
  (bind _distancealongspline (`self.DistanceAlongSpline`))
  (bind _dpressed (`self.DPressed`))
  (bind _stepdistance (`self.StepDistance`))
  (bind _spline (`/Game/BluePrints/BP_Spline.Spline` (`self.SplineTrack`)))
  (`KismetSystemLibrary.Delay` 0.01)
  (if (or _dpressed (`self.APressed`))
    ;[1 1 1] Changing distance along spline
    (`self.K2_SetActorLocation` (`self.PlayerBP`) (`SplineComponent.GetLocationAtDistanceAlongSpline` _spline _distancealongspline "World") false false)
    (if _dpressed
      (`/Engine/EditorBlueprintResources/StandardMacros.CompareFloat` _distancealongspline (`SplineComponent.GetSplineLength` _spline) ; Makes sure player can't change the distance along the spline if the end has been reached
        (:`==`
          _)
        (:`<`
          _))
      (set `self.DistanceAlongSpline` (+ (`self.DistanceAlongSpline`) _stepdistance))
      (else
        (`/Engine/EditorBlueprintResources/StandardMacros.CompareFloat` _distancealongspline ; Makes sure player can't change the distance along the spline if the start has been reached
          (:`>`
            _)
          (:`==`
            _))
        (set `self.DistanceAlongSpline` (- (`self.DistanceAlongSpline`) _stepdistance))))))

(event `Key|A`
  (params (Key :type "Key Structure"))
  ;[1 1 1] Get key input
  (:`Pressed`
    (set `self.APressed` true))
  (:`Released`
    (set `self.APressed` false)))

(event `Key|D`
  (params (Key :type "Key Structure"))
  ;[1 1 1] Get key input
  (:`Pressed`
    (set `self.DPressed` true))
  (:`Released`
    (set `self.DPressed` false)))

(fn `UserConstructionScript`)