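; PlayerShooter is an actor that handles mouse-aimed automatic fire for the BP_Player it finds on BeginPlay.
; Each Tick it sets its own yaw from the player toward the cursor's Visibility trace hit.
; The left mouse button opens and closes a Gate on Tick, where a Delay throttles fire.
; Each shot spawns a Projector above the player, rotated along the direction from player to cursor hit.
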(event `self.ReceiveBeginPlay`
  (bind _returnvalue (`GameplayStatics.GetPlayerController` 0))
  (set `PlayerController.bShowMouseCursor` true _returnvalue)
  (`self.EnableInput` _returnvalue)
  ;[1 1 1] Get Player
  (bind _outactors (`GameplayStatics.GetAllActorsOfClass` "/Game/BluePrints/BP_Player.BP_Player_C"))
  (set `self.Player` (`|GetArrayItem` _outactors)))

(event `self.ReceiveTick`
  (params (DeltaSeconds :type "Float (single-precision)"))
  (bind _returnvalue (`self.K2_GetActorLocation` (`self.Player`)))
  (bind _returnvalue_2 (`KismetMathLibrary.FindLookAtRotation` _returnvalue (`.Location` (`GameplayStatics.BreakHitResult` (`PlayerController.GetHitResultUnderCursorByChannel` (`GameplayStatics.GetPlayerController` 0) "TraceTypeQuery1" true)))))
  (`self.K2_SetActorRotation` (`KismetMathLibrary.MakeRotator` 0.0 0.0 (.yaw _returnvalue_2)))
  (`/Engine/EditorBlueprintResources/StandardMacros.Gate` true :!label _label
    (:`Exit`
      (`KismetSystemLibrary.Delay` 0.2)
      (`|SpawnActorFromClass` "/Game/BluePrints/Projector.Projector_C" (`KismetMathLibrary.MakeTransform` (+ _returnvalue (0.0 0.0 100.0)) _returnvalue_2) "Undefined" "OverrideRootScale" null null))))

(event `Key|LeftMouseButton`
  (params (Key :type "Key Structure"))
  (:`Pressed`
    (goto _label :!via `Open`))
  (:`Released`
    (goto _label :!via `Close`)))

(fn `UserConstructionScript`)