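; BP_GridPlacement is a test Blueprint that computes a grid-snapped mouse position on the XZ plane.
; Every Tick, SnapMouseLocation deprojects player 0's cursor to world space, snaps X and Z to GridSize, and fixes Y at zero.
; The result is not yet applied to anything, and the MainCamera cached on BeginPlay from the first CameraActor found is unused.
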(event `self.ReceiveBeginPlay`
  (bind _outactors (`GameplayStatics.GetAllActorsOfClass` "/Script/Engine.CameraActor"))
  (set `self.MainCamera` (`|GetArrayItem` _outactors)))

(event `self.ReceiveTick`
  (params (DeltaSeconds :type "Float (single-precision)"))
  (`self.SnapMouseLocation` (`self.GridSize`)))

(fn `SnapMouseLocation`
  (params (GridSize :type "Float (double-precision)"))
  (returns (SnappedLocation :type "Vector Structure"))
  (return (`KismetMathLibrary.MakeVector` (`KismetMathLibrary.GridSnap_Float` (.x (`PlayerController.DeprojectMousePositionToWorld` (`GameplayStatics.GetPlayerController` 0))) GridSize) 0.0 (`KismetMathLibrary.GridSnap_Float` (.z (`PlayerController.DeprojectMousePositionToWorld` (`GameplayStatics.GetPlayerController` 0))) GridSize))))

(fn `UserConstructionScript`)